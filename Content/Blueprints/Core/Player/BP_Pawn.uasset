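; BP_Pawn is a player-controlled camera pawn with smoothed movement, stepped yaw rotation and spring arm zoom.
; Input axes shift a desired location along the actor's forward and right vectors and adjust a clamped desired zoom, while rotation actions add fixed yaw steps.
; Tick interpolates location, rotation and arm length toward these targets at separate speeds, moving without sweep collision.
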(event EventTick
  (params (DeltaSeconds :type Float%20%28single-precision%29))
  (bind _springarm (Variables|Default|GetSpringArm))
  ;[0 0.4496 1] Event Tick
  (Variables|/Script/Engine.SpringArmComponent|SetTargetArmLength _springarm (Math|Interpolation|FInterpTo (Variables|/Script/Engine.SpringArmComponent|GetTargetArmLength _springarm) (Variables|Default|GetZoom_Desired) DeltaSeconds (Variables|Default|GetZoomInterpZpeed)))
  (Transformation|SetActorLocation (Math|Interpolation|VInterpTo (Transformation|GetActorLocation) (Variables|Default|GetLocationDesired) DeltaSeconds (Variables|Default|GetMoveInterpSpeed)) false false)
  (Transformation|SetActorRotation (Math|Interpolation|RInterpTo (Transformation|GetActorRotation) (Variables|Default|GetRotationDesired) DeltaSeconds (Variables|Default|GetRotateInterpSpeed))))

(event EventBeginPlay
  (Variables|Default|SetLocationDesired (Transformation|GetActorLocation))
  (Variables|Default|SetZoom_Desired (Variables|/Script/Engine.SpringArmComponent|GetTargetArmLength (Variables|Default|GetSpringArm)))
  (Variables|Default|SetRotationDesired (Transformation|GetActorRotation)))

(event Input|ActionEvents|InputActionInputActionRotationRight
  (params (Key :type Key%20Structure :default "None"))
  (:Pressed
    (Variables|Default|SetRotationDesired (Math|Rotator|CombineRotators (Variables|Default|GetRotationDesired) (Math|Rotator|MakeRotator 0.0 0.0 (Variables|Default|GetRotationRate))))))

(event Input|ActionEvents|InputActionInputActionRotationLeft
  (params (Key :type Key%20Structure :default "None"))
  (:Pressed
    (Variables|Default|SetRotationDesired (Math|Rotator|CombineRotators (Variables|Default|GetRotationDesired) (Math|Rotator|MakeRotator 0.0 0.0 (* (Variables|Default|GetRotationRate) -1.0))))))

(event Input|AxisEvents|InputAxisInputAxisZoom
  (params (AxisValue :type Float%20%28single-precision%29))
  ;[1 1 1] Camera Zoom
  (Variables|Default|SetZoom_Desired (Math|Float|Clamp(Float) (+ (Variables|Default|GetZoom_Desired) (* AxisValue (Variables|Default|GetZoomRate))) (Variables|Default|GetZoomMin) (Variables|Default|GetZoomMax))))

(event Input|AxisEvents|InputAxisInputAxisForward
  (params (AxisValue :type Float%20%28single-precision%29))
  ;[1 1 1] Move Pawn X axis
  (Variables|Default|SetLocationDesired (+ (Variables|Default|GetLocationDesired) (* (* AxisValue (Variables|Default|GetMoveSpeed)) (Transformation|GetActorForwardVector)))))

(event Input|AxisEvents|InputAxisInputAxisRight
  (params (AxisValue :type Float%20%28single-precision%29))
  ;[1 1 1] Move Pawn Y axis
  (Variables|Default|SetLocationDesired (+ (Variables|Default|GetLocationDesired) (* (* AxisValue (Variables|Default|GetMoveSpeed)) (Transformation|GetActorRightVector)))))

(fn ConstructionScript)