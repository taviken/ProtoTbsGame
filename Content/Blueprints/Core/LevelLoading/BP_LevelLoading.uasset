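; BP_LevelLoading switches between streaming levels, keeping track of the active one by name in LevelLoaded.
; On BeginPlay it force-loads the level already stored in LevelLoaded.
; LoadLevel skips repeat requests unless forced, flags the previous streaming level to unload and hide, then flags the new one to load and show.
; A name other than "None" with no matching streaming level prints an on-screen error.
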(event EventBeginPlay
  (CallFunction|LoadLevel (Variables|Default|GetLevelLoaded) true))

(fn ConstructionScript)

(fn LoadLevel
  (params (Level :type String) (Force :type Boolean))
  (bind _returnvalue (Utilities|String|StringToName Level))
  (bind _returnvalue_2 (Class|GameplayStatics|GetStreamingLevel _returnvalue))
  (if (or Force (Utilities|Enum|NotEqual(Enum) Level (Variables|Default|GetLevelLoaded)))
    (Utilities|FlowControl|Sequence
      (:then_0
        (Utilities|IsValid (Class|GameplayStatics|GetStreamingLevel (Utilities|String|StringToName (Variables|Default|GetLevelLoaded)))
          (:Is%20Valid
            (Variables|/Script/Engine.LevelStreaming|SetbShouldBeLoaded (Class|GameplayStatics|GetStreamingLevel (Utilities|String|StringToName (Variables|Default|GetLevelLoaded))) false)
            (Variables|/Script/Engine.LevelStreaming|SetbShouldBeVisible (Class|GameplayStatics|GetStreamingLevel (Utilities|String|StringToName (Variables|Default|GetLevelLoaded))) false))))
      (:then_1
        (Variables|Default|SetLevelLoaded Level)
        (Utilities|IsValid _returnvalue_2
          (:Is%20Valid
            (Variables|/Script/Engine.LevelStreaming|SetbShouldBeLoaded _returnvalue_2 true)
            (Variables|/Script/Engine.LevelStreaming|SetbShouldBeVisible _returnvalue_2 true))
          (:Is%20Not%20Valid
            (if (Utilities|Enum|NotEqual(Enum) (Variables|Default|GetLevelLoaded) "None")
              (Development|PrintString (Utilities|String|Append "Erro Loading Level " (Variables|Default|GetLevelLoaded)) true true "(R=0.000000,G=0.660000,B=1.000000,A=1.000000)" 5.0))))))))