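; BP_Grid is a tile grid actor that builds a square, hexagon or triangle layout in the construction script from center, tile size, count and shape.
; Shape data from DT_GridShapeData supplies the mesh, material and scale for one InstancedStaticMesh, which is cleared and refilled on each spawn.
; Per-shape math snaps the center and derives the bottom-left origin for tile placement.
; Hexagons use doubled, parity-staggered Y indices; triangles flip yaw by index parity.
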(event EventBeginPlay)

(event Collision|EventActorBeginOverlap
  (params (OtherActor :type Actor%20Object%20Reference)))

(event EventTick
  (params (DeltaSeconds :type Float%20%28single-precision%29)))

(fn ConstructionScript
  (CallFunction|SpawnGrid (Transformation|GetActorLocation) (Variables|Default|GetGridTileSize) (Variables|Default|GetGridTileCount) (Variables|Default|GetGridTileShape)))

(fn SpawnGrid
  (params (CenterLocation :type Vector) (TileSize :type Vector) (TileCount :type Vector%202D%20Structure) (Shape :type E_GridShape%20Enum :default "NewEnumerator0"))
  (bind _returnvalue (CallFunction|GetCurrentShapeData))
  (bind (_meshsize _mesh _meshmaterial _flatmesh _flatbordermaterial) (Utilities|Struct|BreakS_GridShapeData _returnvalue))
  (Variables|Default|SetGridCenterLocation CenterLocation)
  (Variables|Default|SetGridTileSize TileSize)
  (Variables|Default|SetGridTileShape Shape)
  (Variables|Default|SetGridTileCount (Math|Vector2D|MakeVector2D (Math|Conversions|ToFloat(Integer) (Math|Float|Round (.x (Variables|Default|GetGridTileCount)))) (Math|Conversions|ToFloat(Integer) (Math|Float|Round (.y (Variables|Default|GetGridTileCount))))))
  (CallFunction|DestroyGrid)
  (Components|StaticMesh|SetStaticMesh (Variables|Default|GetInstancedStaticMesh) _flatmesh)
  (Rendering|Material|SetMaterial (Variables|Default|GetInstancedStaticMesh) 0 _flatbordermaterial)
  (bind (_cemter _bottomleft) (CallFunction|CalculateCenterandBottomLeft))
  (Variables|Default|SetGridCenterLocation _cemter)
  (Variables|Default|SetGridBottomLeftCornerLocation _bottomleft)
  (for _index (range 0 (- (Math|Float|Round (.x (Variables|Default|GetGridTileCount))) 1))
    (LocalVariables|Setx _index)
    (if (Utilities|Enum|NotEqual(Enum) (Variables|Default|GetGridTileShape) "NewEnumerator2")
      (for _index_2 (range 0 (- (Math|Float|Round (.y (Variables|Default|GetGridTileCount))) 1))
        (LocalVariables|Sety _index_2)
        (LocalVariables|SetIndex (Math|Vector2D|MakeVector2D (Math|Conversions|ToFloat(Integer) (LocalVariables|Getx)) (Math|Conversions|ToFloat(Integer) (LocalVariables|Gety))))
        (LocalVariables|SetTileRansform (Math|Transform|MakeTransform (CallFunction|GetTileLocationfromGridIndex (LocalVariables|GetIndex)) (CallFunction|GetTileRotationfromGridIndex (LocalVariables|GetIndex)) (/ (Variables|Default|GetGridTileSize) (.MeshSize (Utilities|Struct|BreakS_GridShapeData (CallFunction|GetCurrentShapeData))))))
        (Components|InstancedStaticMesh|AddInstance (Variables|Default|GetInstancedStaticMesh) (LocalVariables|GetTileRansform) true))
      (else
        (for _index_3 (range (Math|Integer|SelectInt 0 1 (CallFunction|IsIntEven (LocalVariables|Getx))) (- (* (Math|Float|Round (.y (Variables|Default|GetGridTileCount))) 2) 1))
          (LocalVariables|Sety _index_3)
          (Utilities|FlowControl|Sequence
            (:then_0
              (LocalVariables|SetIndex (Math|Vector2D|MakeVector2D (Math|Conversions|ToFloat(Integer) (LocalVariables|Getx)) (Math|Conversions|ToFloat(Integer) (LocalVariables|Gety))))
              (LocalVariables|SetTileRansform (Math|Transform|MakeTransform (CallFunction|GetTileLocationfromGridIndex (LocalVariables|GetIndex)) (CallFunction|GetTileRotationfromGridIndex (LocalVariables|GetIndex)) (/ (Variables|Default|GetGridTileSize) (.MeshSize (Utilities|Struct|BreakS_GridShapeData (CallFunction|GetCurrentShapeData))))))
              (Components|InstancedStaticMesh|AddInstance (Variables|Default|GetInstancedStaticMesh) (LocalVariables|GetTileRansform) true))
            (:then_1
              (Math|Integer|IncrementInt _index_3))))))))

(fn GetCurrentShapeData
  (bind _gridtileshape (Variables|Default|GetGridTileShape))
  (bind _returnvalue (Utilities|String|EnumtoString _gridtileshape))
  (bind _returnvalue_2 (Utilities|GetDataTableRow "/Game/Blueprints/Core/Grid/GridShapes/DT_GridShapeData.DT_GridShapeData" (Utilities|String|StringToName _returnvalue))
    (:then
      _)
    (:RowNotFound
      (Development|PrintString (Utilities|String|Append "Error - Row not found - " _returnvalue) true true "(R=1.000000,G=0.000000,B=0.000000,A=1.000000)" 5.0)))
  (return _returnvalue_2))

(fn DestroyGrid
  (Components|InstancedStaticMesh|ClearInstances (Variables|Default|GetInstancedStaticMesh)))

(fn CalculateCenterandBottomLeft
  (bind _gridtilecount (Variables|Default|GetGridTileCount))
  (switch Utilities|FlowControl|Switch|SwitchonE_GridShape (Variables|Default|GetGridTileShape)
    (:NewEnumerator1
      (Variables|Default|SetCenter (CallFunction|SnapVectortoVector (Variables|Default|GetGridCenterLocation) (Variables|Default|GetGridTileSize)))
      (return (Variables|Default|GetCenter) (- (Variables|Default|GetCenter) (* (/ (- (Variables|Default|GetGridTileCount) (Math|Vector2D|MakeVector2D (Math|Float|SelectFloat 0.0 1.0 (CallFunction|IsFloatEven (.x _gridtilecount))) (Math|Float|SelectFloat 0.0 1.0 (CallFunction|IsFloatEven (.y _gridtilecount))))) 2.0) (Variables|Default|GetGridTileSize)))))
    (:NewEnumerator2
      (Variables|Default|SetCenter (CallFunction|SnapVectortoVector (Variables|Default|GetGridCenterLocation) (* (Variables|Default|GetGridTileSize) "1.500000,1.000000,1.000000")))
      (return (Variables|Default|GetCenter) (- (Variables|Default|GetCenter) (CallFunction|SnapVectortoVector (* (/ (Variables|Default|GetGridTileCount) "(X=3.000000,Y=2.000000)") (Variables|Default|GetGridTileSize)) (* (Variables|Default|GetGridTileSize) "1.500000,1.000000,1.000000")))))
    (:NewEnumerator3
      (Variables|Default|SetCenter (CallFunction|SnapVectortoVector (Variables|Default|GetGridCenterLocation) (* (Variables|Default|GetGridTileSize) "2.000000,1.000000,1.000000")))
      (return (Variables|Default|GetCenter) (- (Variables|Default|GetCenter) (CallFunction|SnapVectortoVector (* (/ (- (Variables|Default|GetGridTileCount) (Math|Vector2D|MakeVector2D 1.0 1.0)) "(X=2.000000,Y=4.000000)") (Variables|Default|GetGridTileSize)) (* (Variables|Default|GetGridTileSize) "2.000000,1.000000,1.000000")))))))

(fn GetTileRotationfromGridIndex
  (params (GridIndex :type Vector%202D%20Structure))
  (if (Utilities|Enum|Equal(Enum) (Variables|Default|GetGridTileShape) "NewEnumerator3")
    (return (Math|Rotator|MakeRotator 0.0 0.0 (+ (Math|Float|SelectFloat 1.8e+02 0.0 (CallFunction|IsFloatEven (.x GridIndex))) (Math|Float|SelectFloat 1.8e+02 0.0 (CallFunction|IsFloatEven (.y GridIndex))))))
    (else
      (return ""))))

(fn GetTileLocationfromGridIndex
  (params (GridIndex :type Vector%202D%20Structure))
  (return (+ (Variables|Default|GetGridBottomLeftCornerLocation) (* (Variables|Default|GetGridTileSize) (* GridIndex (Utilities|Select :Index (Variables|Default|GetGridTileShape) :NewEnumerator0 "(X=0.000000,Y=0.000000)" :NewEnumerator1 "(X=1.000000,Y=1.000000)" :NewEnumerator2 "(X=0.750000,Y=0.500000)" :NewEnumerator3 "(X=1.000000,Y=0.500000)"))))))